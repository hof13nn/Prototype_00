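; A one-shot downstairs path trigger that opens when the overlapping player holds the key tag set in PassTag.
; Without the key it shows a timed clue naming it.
; With it, it removes the decal, refills the player's light, shows a confirmation and respawns PlayerStart at the trigger box as a checkpoint.
; A FlipFlop re-entered on timeline finish then cycles Cube01 vertically indefinitely, with a delay and door sound before each move.
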(event Custom|RemoveWidget
  ;[1 1 1] Activate Path
  (Widget|RemovefromParent (Variables|Default|GetClueWidget)))

(event Custom|DeleteWidget
  ;[1 1 1] Create Widget with Clue
  (Widget|RemovefromParent (Variables|Default|GetClueWidget)))

(event EventBeginPlay)

(event Collision|EventActorBeginOverlap
  (params (OtherActor :type Actor%20Object%20Reference))
  (bind _cube01 (Variables|Default|GetCube01))
  (bind _relativelocation (Variables|/Script/Engine.SceneComponent|GetRelativeLocation _cube01))
  (if (not (Variables|Default|GetbIsActivated))
    (bind _asp00_player_character (Utilities|Casting|CastToP00_PlayerCharacter OtherActor))
    (if (Class|P00ActionHandlerComponent|HasKeyTag (Class|P00PlayerCharacter|GetActionComponent _asp00_player_character) (Variables|Default|GetPassTag))
      (Variables|Default|SetbIsActivated true)
      (Components|DestroyComponent (Variables|Default|GetDecal))
      ;[1 1 1] Activate Path
      (Class|P00PlayerCharacter|ResetLighttoMax _asp00_player_character)
      (Utilities|FlowControl|Sequence
        (:then_0
          (Utilities|IsValid (Variables|Default|GetClueWidget)
            (:Is%20Valid
              (Widget|RemovefromParent (Variables|Default|GetClueWidget)))
            (:Is%20Not%20Valid
              _))
          (bind _returnvalue (UserInterface|CreateWidget "/Game/Prototype_00/BPs/UI/Pure_BP/WBP_TriggerClue.WBP_TriggerClue_C"))
          (bind _output_get (Variables|Default|SetClueWidget _returnvalue))
          (bind _result (CallFunction|FormatTagtoText "{Text} Key Opened the Path"))
          (Default|SetClueText _output_get (Utilities|Text|FormatText " {Text} Key Opened the Path" _result))
          (UserInterface|Viewport|AddtoViewport _output_get 0)
          (Utilities|Time|SetTimerbyEvent (delegate Custom|RemoveWidget) 3.0)
          (bind _returnvalue_2 (Actor|GetActorOfClass "/Script/Engine.PlayerStart"))
          (Utilities|IsValid _returnvalue_2
            (:Is%20Valid
              (Actor|DestroyActor _returnvalue_2)
              (Game|SpawnActorfromClass "/Script/Engine.PlayerStart" (Math|Transform|MakeTransform (Transformation|GetWorldLocation (Variables|Default|GetBox)) (Transformation|GetActorRotation _asp00_player_character) "1.000000,1.000000,1.000000") "Undefined" "MultiplyWithRoot" 0 0))))
        (:then_1
          (Utilities|FlowControl|FlipFlop :!label _label
            (:A
              (Utilities|FlowControl|Delay 3.0)
              (Audio|PlaySoundatLocation "/Game/Prototype_00/Sounds/Door/SC_DoorOpen.SC_DoorOpen" (Transformation|GetActorLocation) "0, 0, 0" 1.0 1.0 0.0 0 0 0 0)
              (bind _vertical_value (Timeline|Cube01_TL Play)
                (:Update
                  (Transformation|SetRelativeLocation _cube01 (Math|Vector|MakeVector (.x _relativelocation) (.y _relativelocation) _vertical_value) false false))
                (:Finished
                  (goto _label))))
            (:B
              (Utilities|FlowControl|Delay 3.0)
              (Audio|PlaySoundatLocation "/Game/Prototype_00/Sounds/Door/SC_DoorOpen.SC_DoorOpen" (Transformation|GetActorLocation) "0, 0, 0" 1.0 1.0 0.0 0 0 0 0)
              (Timeline|Cube01_TL Reverse)))))
      (else
        ;[1 1 1] Create Widget with Clue
        (bind _returnvalue_3 (UserInterface|CreateWidget "/Game/Prototype_00/BPs/UI/Pure_BP/WBP_TriggerClue.WBP_TriggerClue_C"))
        (bind _output_get_2 (Variables|Default|SetClueWidget _returnvalue_3))
        (bind _result_2 (CallFunction|FormatTagtoText "Find {Text} Key to open the Path"))
        (Default|SetClueText _output_get_2 (Utilities|Text|FormatText "Find {Text} Key to Open the Path" _result_2))
        (UserInterface|Viewport|AddtoViewport _output_get_2 0)
        (Utilities|Time|SetTimerbyEvent (delegate Custom|DeleteWidget) 5.0)))))

(event EventTick
  (params (DeltaSeconds :type Float%20%28single-precision%29)))

(fn ConstructionScript)

(fn FormatTagtoText
  (params (FromatTemplate :type Text))
  (return (Utilities|Text|ToText(String) (Utilities|String|Replace (Utilities|String|ToString(Text) (Utilities|Text|ToText(Name) (GameplayTags|GetTagName (Variables|Default|GetPassTag)))) "Key."))))