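; Level exit actor that ends the game when the player overlaps it carrying the required key tags.
; On overlap it checks the player's ActionComponent for PassTags; a match plays the unlock sound, shows the win screen, pauses, then calls Delay before QuitGame.
; Otherwise it shows a timed clue widget naming the missing key, derived from PassTag by stripping the "Key." prefix.
; The Niagara activation node is never executed.
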(event Custom|DeleteWidget
  ;[1 1 1] Create Widget with Clue
  (Widget|RemovefromParent (Variables|Default|GetClueWidget)))

(event Collision|EventActorBeginOverlap
  (params (OtherActor :type Actor%20Object%20Reference))
  (bind _asp00_player_character (Utilities|Casting|CastToP00_PlayerCharacter OtherActor))
  ;[1 1 1] Activate Path
  (if (Class|P00ActionHandlerComponent|HasKeyTags (Class|P00PlayerCharacter|GetActionComponent _asp00_player_character) (Variables|Default|GetPassTags))
    (Utilities|FlowControl|Sequence
      (:then_0
        (Audio|PlaySoundatLocation "/Game/Prototype_00/Sounds/Door/SC_UnlockedSound.SC_UnlockedSound" (Transformation|GetActorLocation) "0, 0, 0" 1.0 1.0 0.0 0 0 0 0))
      (:then_1
        (bind _returnvalue (UserInterface|CreateWidget "/Game/Prototype_00/BPs/UI/Pure_BP/WBP_WinScreen.WBP_WinScreen_C"))
        (UserInterface|Viewport|AddtoViewport _returnvalue 0)
        (Game|SetGamePaused true)
        (Utilities|FlowControl|Delay 3.0)
        (Game|QuitGame 0 "Quit" false)))
    (else
      ;[1 1 1] Create Widget with Clue
      (bind _returnvalue_2 (UserInterface|CreateWidget "/Game/Prototype_00/BPs/UI/Pure_BP/WBP_TriggerClue.WBP_TriggerClue_C"))
      (bind _output_get (Variables|Default|SetClueWidget _returnvalue_2))
      (bind _result (CallFunction|FormatTagtoText "Find {Text} Key to open the Path"))
      (Default|SetClueText _output_get (Utilities|Text|FormatText "Find {Text} Key to Open the Path" _result))
      (UserInterface|Viewport|AddtoViewport _output_get 0)
      (Utilities|Time|SetTimerbyEvent (delegate Custom|DeleteWidget) 3.0))))

(fn ConstructionScript)

(fn FormatTagtoText
  (params (FromatTemplate :type Text))
  (return (Utilities|Text|ToText(String) (Utilities|String|Replace (Utilities|String|ToString(Text) (Utilities|Text|ToText(Name) (GameplayTags|GetTagName (Variables|Default|GetPassTag)))) "Key."))))